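; Kraken enemy character that roams, hunts seen pawns and ends the run when it catches the rover.
; It loops AI moves to random reachable points, while Tick checks the pawn stored by PawnSensing and, when in range, closes in to roar and play an attack montage.
; Hitbox overlap with BP_Rover shows the caught widget, pauses and opens the Dead level.
; A Speedup function incrementally raises walk speed.
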(event OnSeePawn(PawnSensing)
  (params (Pawn :type Pawn%20Object%20Reference))
  ;[1 1 1] Event See Player
  (Variables|Default|SetChasingPawn Pawn))

(event OnComponentBeginOverlap(Hitbox)
  (params (OverlappedComponent :type Primitive%20Component%20Object%20Reference) (OtherActor :type Actor%20Object%20Reference) (OtherComp :type Primitive%20Component%20Object%20Reference) (OtherBodyIndex :type Integer) (bFromSweep :type Boolean) (SweepResult :type Hit%20Result%20Structure%20%28by%20ref%29))
  ;[1 1 1] Player Death
  (Utilities|Casting|CastToBP_Rover OtherActor)
  (bind _returnvalue (UserInterface|CreateWidget "/Game/Widgets/WP_Caught.WP_Caught_C"))
  (UserInterface|Viewport|AddtoViewport _returnvalue 0)
  (Game|SetGamePaused true)
  (Utilities|FlowControl|Delay 2.0)
  (Game|SetGamePaused false)
  (Game|OpenLevel(byObjectReference) "/Game/Moon_Maps/Dead.Dead"))

(event Custom|Roam
  ;[1 1 1] Roam
  (if (not (Variables|Default|GetisRoaming))
    (if (not (Variables|Default|GetisAttacking))
      (Variables|Default|SetisRoaming true)
      (AI|AIMoveTo self (.RandomLocation (AI|Navigation|GetRandomReachablePointinRadius (Transformation|GetActorLocation) 8e+03 0 0)) 0 2.5e+02 false
        (:OnSuccess
          _)
        (:OnFail
          _))
      (Utilities|FlowControl|Delay 3.0)
      (Variables|Default|SetisRoaming false)
      (CallFunction|Roam))))

(event Custom|UpdatePawnChase
  ;[1 1 1] Update Pawn Chase
  (Utilities|IsValid (Variables|Default|GetChasingPawn)
    (:Is%20Valid
      (if (<= (Math|Vector|Distance(Vector) (Transformation|GetActorLocation (Variables|Default|GetChasingPawn)) (Transformation|GetActorLocation)) 1e+04)
        (if (not (Variables|Default|GetisAttacking))
          (Variables|Default|SetisAttacking true)
          (AI|Navigation|StopMovement (AI|GetAIController self))
          (AI|AIMoveTo self "0, 0, 0" (Variables|Default|GetChasingPawn) 1.6e+03 false
            (:OnSuccess
              (Audio|PlaySoundatLocation "/Game/SoundFx/MonsterRoars.MonsterRoars" (Transformation|GetActorLocation) "0, 0, 0" 1.0 1.0 0.0 0 0 0 0)
              (bind _returnvalue (Animation|PlayAnimMontage "/Game/Blueprints/ShortAttackMontage.ShortAttackMontage" 1.0 "None"))
              (Utilities|FlowControl|Delay _returnvalue))
            (:OnFail
              _))
          (Variables|Default|SetisAttacking false)
          (CallFunction|Roam))))
    (:Is%20Not%20Valid
      (CallFunction|Roam))))

(event EventTick
  (params (DeltaSeconds :type Float%20%28single-precision%29))
  ;[1 1 1] Tick Event
  (CallFunction|UpdatePawnChase))

(event EventAsyncPhysicsTick
  (params (DeltaSeconds :type Float%20%28single-precision%29) (SimSeconds :type Float%20%28single-precision%29))
  ;[1 1 1] Tick Event
  (Utilities|FlowControl|Delay (Math|Random|RandomFloatinRange 3.0 6.0))
  (Audio|PlaySoundatLocation "/Game/SoundFx/MonsterAngry.MonsterAngry" (Transformation|GetActorLocation) "0, 0, 0" 1.0 1.0 0.0 0 0 0 0))

(event EventBeginPlay
  ;[1 1 1] Begin Play
  (Audio|PlaySound2D "/Game/SoundFx/MonsterFirstChase.MonsterFirstChase" 1.0 1.0 0.0 0 0)
  (CallFunction|Roam))

(fn ConstructionScript)

(fn Speedup
  (bind _charactermovement (Variables|Character|GetCharacterMovement))
  (Variables|/Script/Engine.CharacterMovementComponent|SetMaxWalkSpeed _charactermovement (+ (Class|MovementComponent|GetMaxSpeed _charactermovement) 5e+01)))