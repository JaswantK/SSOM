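; KrakenStasis is a dormant kraken stand-in that breathes near the rover, then becomes a live AI kraken when the rover leaves.
; When BP_Rover overlaps the actor, it plays five monster breathing sounds at the stasis location, spaced by staggered delays.
; When the rover exits the Sphere component, the actor destroys itself, spawns BP_KrakenAI at SpawnTransform and gives it a default controller.
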(event OnComponentEndOverlap(Sphere)
  (params (OverlappedComponent :type Primitive%20Component%20Object%20Reference) (OtherActor :type Actor%20Object%20Reference) (OtherComp :type Primitive%20Component%20Object%20Reference) (OtherBodyIndex :type Integer))
  (Utilities|Casting|CastToBP_Rover OtherActor)
  (Actor|DestroyActor)
  (bind _returnvalue (Game|SpawnActorfromClass "/Game/Blueprints/BP_KrakenAI.BP_KrakenAI_C" (Variables|Default|GetSpawn%20Transform) "AdjustIfPossibleButAlwaysSpawn" "MultiplyWithRoot" 0 0))
  (Pawn|SpawnDefaultController _returnvalue))

(event Collision|EventActorBeginOverlap
  (params (OtherActor :type Actor%20Object%20Reference))
  (Utilities|Casting|CastToBP_Rover OtherActor)
  (Audio|PlaySoundatLocation "/Game/SoundFx/MonsterBreathing.MonsterBreathing" (Variables|Default|GetStasisKrakenLocation) "0, 0, 0" 1.0 1.0 0.0 0 0 0 0)
  (Utilities|FlowControl|Delay 4.5)
  (Audio|PlaySoundatLocation "/Game/SoundFx/MonsterBreathing.MonsterBreathing" (Variables|Default|GetStasisKrakenLocation) "0, 0, 0" 1.0 1.0 0.0 0 0 0 0)
  (Utilities|FlowControl|Delay 5.0)
  (Audio|PlaySoundatLocation "/Game/SoundFx/MonsterBreathing.MonsterBreathing" (Variables|Default|GetStasisKrakenLocation) "0, 0, 0" 1.0 1.0 0.0 0 0 0 0)
  (Utilities|FlowControl|Delay 4.0)
  (Audio|PlaySoundatLocation "/Game/SoundFx/MonsterBreathing.MonsterBreathing" (Variables|Default|GetStasisKrakenLocation) "0, 0, 0" 1.0 1.0 0.0 0 0 0 0)
  (Utilities|FlowControl|Delay 5.0)
  (Audio|PlaySoundatLocation "/Game/SoundFx/MonsterBreathing.MonsterBreathing" (Variables|Default|GetStasisKrakenLocation) "0, 0, 0" 1.0 1.0 0.0 0 0 0 0))

(fn ConstructionScript)