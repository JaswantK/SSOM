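; BP_Rover is the player-driven rover vehicle, with throttle, brake, steering and a pitch-limited mouse camera.
; It shows a mission widget after a short delay, exposes functions to update mission text and scanned-site count, and opens an options menu on Tab or Escape.
; Reset input lifts a stuck rover, and another teleports it to fixed Lander coordinates.
; Damage lowers clamped health, but the death check is unconnected.
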(event EventBeginPlay
  (bind _returnvalue (Game|GetPlayerCameraManager 0))
  ;[1 1 1] Limit Camera from being too close
  (Variables|/Script/Engine.PlayerCameraManager|SetViewPitchMax _returnvalue 1.8)
  (Variables|/Script/Engine.PlayerCameraManager|SetViewPitchMin _returnvalue -25.0)
  (Utilities|FlowControl|Delay 4.9)
  (bind _returnvalue_2 (UserInterface|CreateWidget "/Game/Widgets/WP_Mission.WP_Mission_C" (Game|GetPlayerController 0)))
  (bind _output_get (Variables|Default|SetMissionWidget _returnvalue_2))
  (UserInterface|Viewport|AddtoViewport _output_get 0))

(event Game|Damage|EventAnyDamage
  (params (Damage :type Float%20%28single-precision%29) (DamageType :type Damage%20Type%20Object%20Reference) (InstigatedBy :type Controller%20Object%20Reference) (DamageCauser :type Actor%20Object%20Reference))
  ;[1 1 1] Recieving Damage
  (if (not (Variables|Default|GetisDead%20?))
    (bind _output_get (Variables|Default|SetHealth (Math|Float|Clamp(Float) (- (Variables|Default|GetHealth) Damage) 0.0 (Variables|Default|GetMaxHealth))))))

(event Input|ActionEvents|InputActionResetVehicle
  (params (Key :type Key%20Structure))
  ;[1 1 1] Teleport Vehicle if stuck
  (:Pressed
    (Transformation|Teleport (+ (Transformation|GetActorLocation) "0.000000,0.000000,120.000000") (Math|Rotator|MakeRotator 0.0 0.0 (.yaw (Transformation|GetActorRotation))))))

(event Input|ActionEvents|InputActionTeleporttoLander
  (params (Key :type Key%20Structure))
  ;[1 1 1] Teleport Vehicle if stuck
  (:Released
    (Transformation|Teleport "40735.000000,51266.000000,3689.000000" (Math|Rotator|MakeRotator 0.0 0.0 (.yaw (Transformation|GetActorRotation))))))

(event Input|AxisEvents|InputAxisMouseUp/Down
  (params (AxisValue :type Float%20%28single-precision%29))
  ;[1 1 1] Mouse Control
  (Pawn|Input|AddControllerPitchInput (* AxisValue -1.0)))

(event Input|AxisEvents|InputAxisThrottle
  (params (AxisValue :type Float%20%28single-precision%29))
  ;[1 1 1] Move Forward
  (Class|ChaosVehicleMovementComponent|SetThrottleInput (Variables|Default|GetVehicleMovementComponent) AxisValue))

(event Input|AxisEvents|InputAxisBrake
  (params (AxisValue :type Float%20%28single-precision%29))
  ;[1 1 1] Move Backward
  (Class|ChaosVehicleMovementComponent|SetBrakeInput (Variables|Default|GetVehicleMovementComponent) AxisValue))

(event Input|AxisEvents|InputAxisMoveRight
  (params (AxisValue :type Float%20%28single-precision%29))
  ;[1 1 1] Move Left & Right
  (Class|ChaosVehicleMovementComponent|SetSteeringInput (Variables|Default|GetVehicleMovementComponent) AxisValue))

(event Input|AxisEvents|InputAxisMouseLeft/Right
  (params (AxisValue :type Float%20%28single-precision%29))
  ;[1 1 1] Mouse Control
  (Pawn|Input|AddControllerYawInput AxisValue))

(event Input|KeyboardEvents|Escape
  (params (Key :type Key%20Structure))
  (bind _returnvalue (Game|GetPlayerController 0))
  (:Pressed
    (bind _returnvalue_2 (UserInterface|CreateWidget "/Game/Widgets/OptionsMenu.OptionsMenu_C" _returnvalue))
    (bind _output_get (Variables|Default|SetOptions%20Widget _returnvalue_2))
    (UserInterface|Viewport|AddtoViewport _output_get 0)
    (Input|SetInputModeGameandUI _returnvalue 0 "DoNotLock" false false)
    (Variables|/Script/Engine.PlayerController|SetbShowMouseCursor _returnvalue true)))

(event Input|KeyboardEvents|Tab
  (params (Key :type Key%20Structure))
  (bind _returnvalue (Game|GetPlayerController 0))
  (:Pressed
    (bind _returnvalue_2 (UserInterface|CreateWidget "/Game/Widgets/OptionsMenu.OptionsMenu_C" _returnvalue))
    (bind _output_get (Variables|Default|SetOptions%20Widget _returnvalue_2))
    (UserInterface|Viewport|AddtoViewport _output_get 0)
    (Input|SetInputModeGameandUI _returnvalue 0 "DoNotLock" false false)
    (Variables|/Script/Engine.PlayerController|SetbShowMouseCursor _returnvalue true)))

(fn ConstructionScript)

(fn UpdateMission
  (params (currentMission :type String))
  (Variables|Default|SetcurrentMission currentMission)
  (Rendering|Components|TextRender|SetText (Variables|/Game/Widgets/WP_Mission.WP_Mission_C|GetcurrentMissionText (Variables|Default|GetMissionWidget)) (Utilities|Text|ToText(String) (Variables|Default|GetcurrentMission))))

(fn UpdateScannedSites
  (Variables|Default|SetscannedSites (+ (Variables|Default|GetscannedSites) 1)))